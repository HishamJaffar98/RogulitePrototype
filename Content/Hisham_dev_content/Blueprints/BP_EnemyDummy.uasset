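; BP_EnemyDummy is a target dummy enemy with health and a floating health bar widget, damaged by the player's dash.
; Overlapping its capsule with a dashing BP_ThirdPersonCharacter subtracts that character's energy or normal dash damage, depending on energy mode.
; Every tick it updates the bar's fill, rotates the widget to face the player camera, and destroys itself once health reaches zero.
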(event OnComponentBeginOverlap(CapsuleComponent)
  (params (OverlappedComponent :type Primitive%20Component%20Object%20Reference) (OtherActor :type Actor%20Object%20Reference) (OtherComp :type Primitive%20Component%20Object%20Reference) (OtherBodyIndex :type Integer) (bFromSweep :type Boolean) (SweepResult :type Hit%20Result%20Structure%20%28by%20ref%29))
  (bind _asbp_third_person_character (Utilities|Casting|CastToBP_ThirdPersonCharacter OtherActor))
  (Variables|Default|SetplayerCharacterReference _asbp_third_person_character)
  (if (and (Variables|/Game/ThirdPerson/Blueprints/BP_ThirdPersonCharacter.BP_ThirdPersonCharacter_C|GetisDashing (Variables|Default|GetplayerCharacterReference)) (Variables|/Game/ThirdPerson/Blueprints/BP_ThirdPersonCharacter.BP_ThirdPersonCharacter_C|GetisEnergyMode (Variables|Default|GetplayerCharacterReference)))
    (CallFunction|DecrementHealth (Variables|/Game/ThirdPerson/Blueprints/BP_ThirdPersonCharacter.BP_ThirdPersonCharacter_C|GetenergyDashingDamage (Variables|Default|GetplayerCharacterReference)))
    (elif (Variables|/Game/ThirdPerson/Blueprints/BP_ThirdPersonCharacter.BP_ThirdPersonCharacter_C|GetisDashing (Variables|Default|GetplayerCharacterReference))
      (CallFunction|DecrementHealth (Variables|/Game/ThirdPerson/Blueprints/BP_ThirdPersonCharacter.BP_ThirdPersonCharacter_C|GetnormalDashingDamage (Variables|Default|GetplayerCharacterReference))))))

(event EventBeginPlay)

(event Collision|EventActorBeginOverlap
  (params (OtherActor :type Actor%20Object%20Reference)))

(event EventTick
  (params (DeltaSeconds :type Float%20%28single-precision%29))
  (Utilities|FlowControl|Sequence
    (:then_0
      (CallFunction|SetHealthBar (Variables|Default|GetHealthBarWidget)))
    (:then_1
      (if (<= (Variables|Default|GetHealth) 0.0)
        (Actor|DestroyActor)))))

(fn ConstructionScript)

(fn SetHealthBar
  (params (self2 :type Scene%20Component%20Object%20Reference))
  (bind _aswbp_health_bar (Utilities|Casting|CastToWBP_HealthBar (UserInterface|GetWidget (Variables|Default|GetHealthBarWidget))))
  (Progress|SetPercent (Variables|/Game/Hisham_dev_content/UI/WBP_HealthBar.WBP_HealthBar_C|GetHealthBar _aswbp_health_bar) (/ (Variables|Default|GetHealth) 1e+02))
  (Transformation|SetWorldRotation self2 (Math|Rotator|FindLookatRotation (Transformation|GetWorldLocation (Variables|Default|GetHealthBarWidget)) (Transformation|GetWorldLocation (Variables|/Script/Engine.PlayerCameraManager|GetTransformComponent (Game|GetPlayerCameraManager 0)))) false false))

(fn DecrementHealth
  (params (Damage :type Float%20%28double-precision%29))
  (Variables|Default|SetHealth (- (Variables|Default|GetHealth) Damage))
  (return))
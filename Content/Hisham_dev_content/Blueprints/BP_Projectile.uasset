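; BP_Projectile is a projectile that damages BP_EnemyTest enemies and destroys itself on impact.
; Its sphere hit event ignores BP_ThirdPersonCharacter and destroys the projectile on any other non-enemy actor.
; On an enemy hit, player 0's energy mode selects normal or energy-mode damage for DecrementHealth.
; It then has the player character spawn an energy point at the enemy's transform before destroying itself.
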(event OnComponentHit(Sphere)
  (params (HitComponent :type Primitive%20Component%20Object%20Reference) (OtherActor :type Actor%20Object%20Reference) (OtherComp :type Primitive%20Component%20Object%20Reference) (NormalImpulse :type Vector :default "0, 0, 0") (Hit :type Hit%20Result%20Structure%20%28by%20ref%29))
  (Utilities|Casting|CastToBP_ThirdPersonCharacter OtherActor
    (:CastFailed
      (bind _asbp_enemy_test (Utilities|Casting|CastToBP_EnemyTest OtherActor)
        (:then
          (Variables|Default|SetEnemyHitReference _asbp_enemy_test)
          (bind _asbp_third_person_character (Utilities|Casting|CastToBP_ThirdPersonCharacter (Game|GetPlayerCharacter 0)))
          (if (Variables|/Game/ThirdPerson/Blueprints/BP_ThirdPersonCharacter.BP_ThirdPersonCharacter_C|GetisEnergyMode _asbp_third_person_character)
            (Default|DecrementHealth (Variables|Default|GetEnemyHitReference) (Variables|Default|GetProjectileEnergyModeDamage))
            (bind _asbp_third_person_character_2 (Utilities|Casting|CastToBP_ThirdPersonCharacter (Game|GetPlayerCharacter 0)))
            (Default|SpawnEnergyPoint _asbp_third_person_character_2 (Transformation|GetActorTransform (Variables|Default|GetEnemyHitReference)))
            (Actor|DestroyActor)
            (else
              (Default|DecrementHealth (Variables|Default|GetEnemyHitReference) (Variables|Default|GetProjectileDamage))
              (bind _asbp_third_person_character_3 (Utilities|Casting|CastToBP_ThirdPersonCharacter (Game|GetPlayerCharacter 0)))
              (Default|SpawnEnergyPoint _asbp_third_person_character_3 (Transformation|GetActorTransform (Variables|Default|GetEnemyHitReference)))
              (Actor|DestroyActor))))
        (:CastFailed
          (Actor|DestroyActor))))))

(event EventBeginPlay)

(event Collision|EventActorBeginOverlap
  (params (OtherActor :type Actor%20Object%20Reference)))

(event EventTick
  (params (DeltaSeconds :type Float%20%28single-precision%29)))

(fn ConstructionScript)
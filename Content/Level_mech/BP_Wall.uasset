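; BP_Wall is a breakable wall that BP_ThirdPersonCharacter destroys by dashing into it.
; A hit from the dashing character switches the Box to OverlapAllDynamic, so it stops blocking.
; An overlap while dashing sets a one-shot destroyed flag, prints a debug string and plays AM_WallDestroy on the skeletal mesh.
; The actor destroys itself when that montage completes.
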(event OnComponentHit(Box)
  (params (HitComponent :type Primitive%20Component%20Object%20Reference) (OtherActor :type Actor%20Object%20Reference) (OtherComp :type Primitive%20Component%20Object%20Reference) (NormalImpulse :type Vector :default "0, 0, 0") (Hit :type Hit%20Result%20Structure%20%28by%20ref%29))
  (bind _asbp_third_person_character (Utilities|Casting|CastToBP_ThirdPersonCharacter OtherActor))
  (if (Variables|/Game/ThirdPerson/Blueprints/BP_ThirdPersonCharacter.BP_ThirdPersonCharacter_C|GetisDashing _asbp_third_person_character)
    (Collision|SetCollisionProfileName (Variables|Default|GetBox) "OverlapAllDynamic" false :!class /Script/Engine.PrimitiveComponent)))

(event OnComponentBeginOverlap(Box)
  (params (OverlappedComponent :type Primitive%20Component%20Object%20Reference) (OtherActor :type Actor%20Object%20Reference) (OtherComp :type Primitive%20Component%20Object%20Reference) (OtherBodyIndex :type Integer) (bFromSweep :type Boolean) (SweepResult :type Hit%20Result%20Structure%20%28by%20ref%29))
  (bind _asbp_third_person_character (Utilities|Casting|CastToBP_ThirdPersonCharacter OtherActor))
  (if (Variables|/Game/ThirdPerson/Blueprints/BP_ThirdPersonCharacter.BP_ThirdPersonCharacter_C|GetisDashing _asbp_third_person_character)
    (if (not (Variables|Default|GetisWallDestroyed))
      (Variables|Default|SetisWallDestroyed true)
      (Development|PrintString "Hello")
      (Animation|Montage|PlayMontage (Variables|Default|GetSkeletalMesh) "/Game/Level_mech/AM_WallDestroy.AM_WallDestroy" 1.0 0.0 "Default"
        (:OnCompleted
          (Actor|DestroyActor))))))

(event EventBeginPlay)

(event Collision|EventActorBeginOverlap
  (params (OtherActor :type Actor%20Object%20Reference)))

(event EventTick
  (params (DeltaSeconds :type Float%20%28single-precision%29)))

(fn ConstructionScript)
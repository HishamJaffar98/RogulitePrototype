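; BP_EnemyTest is an enemy test Blueprint that shows a world-placed health bar above or on itself, turned toward the player's camera.
; Every Tick it calls SetHealthBar, which casts the widget component's widget to WBP_HealthBar and sets the bar's percent from Health, assuming a maximum of 100.
; The same function billboards the widget component with a look-at rotation toward player 0's camera manager.
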(event EventBeginPlay)

(event Collision|EventActorBeginOverlap
  (params (OtherActor :type Actor%20Object%20Reference)))

(event EventTick
  (params (DeltaSeconds :type Float%20%28single-precision%29))
  (CallFunction|SetHealthBar (Variables|Default|GetHealthBarWidget)))

(fn ConstructionScript)

(fn SetHealthBar
  (params (self2 :type Scene%20Component%20Object%20Reference))
  (bind _aswbp_health_bar (Utilities|Casting|CastToWBP_HealthBar (UserInterface|GetWidget (Variables|Default|GetHealthBarWidget))))
  (Progress|SetPercent (Variables|/Game/WBP_HealthBar.WBP_HealthBar_C|GetHealthBar _aswbp_health_bar) (/ (Variables|Default|GetHealth) 1e+02))
  (Transformation|SetWorldRotation self2 (Math|Rotator|FindLookatRotation (Transformation|GetWorldLocation (Variables|Default|GetHealthBarWidget)) (Transformation|GetWorldLocation (Variables|/Script/Engine.PlayerCameraManager|GetTransformComponent (Game|GetPlayerCameraManager 0)))) false false))